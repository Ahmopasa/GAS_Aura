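; Field System actor that sets off a one-shot physics explosion at its own location as soon as play begins, for breaking destructible objects.
; Explode first applies an external cluster strain field through a radial falloff sphere with no attenuation to fracture geometry clusters.
; It then applies a linear force field from a radial vector centered on the actor to push the pieces outward.
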(event EventBeginPlay
  (CallFunction|Explode))

(fn ConstructionScript)

(fn Explode
  (Class|FieldSystemComponent|ApplyPhysicsField (Variables|Field|GetFieldSystemComponent) true "Field_ExternalClusterStrain" 0 (Field|SetRadialFalloff (Variables|Default|GetRadialFalloff) 1e+06 0.8 1.0 0.0 2e+02 (Transformation|GetActorLocation) "Field_FallOff_None"))
  (Class|FieldSystemComponent|ApplyPhysicsField (Variables|Field|GetFieldSystemComponent) true "Field_LinearForce" 0 (Field|SetRadialVector (Variables|Default|GetRadialVector) 5e+08 (Transformation|GetActorLocation))))