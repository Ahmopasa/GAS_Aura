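; Breakable actor built on a Chaos Geometry Collection that shatters when hit and then cleans itself up.
; On component hit it stores the other actor as BPFirebolt and, if valid, runs HandlingExplosion.
; That function plays a rock sound and spawns BP_FieldSystem at that actor's location.
; A Chaos break event gives the breakable a short lifespan so it is destroyed shortly afterwards.
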(event OnChaosBreakEvent(GeometryCollection)
  (params (BreakEvent :type Chaos%20Break%20Event%20Structure%20%28by%20ref%29))
  ;[1 1 1] Handling of Destruction
  (Actor|SetLifeSpan 3.0))

(event OnComponentHit(GeometryCollection)
  (params (HitComponent :type Primitive%20Component%20Object%20Reference) (OtherActor :type Actor%20Object%20Reference) (OtherComp :type Primitive%20Component%20Object%20Reference) (NormalImpulse :type Vector :default "0, 0, 0") (Hit :type Hit%20Result%20Structure%20%28by%20ref%29))
  ;[1 1 1] Handling of Destruction
  (bind _output_get (Variables|Default|SetBP_Firebolt OtherActor))
  (Utilities|IsValid _output_get
    (:Is%20Valid
      (CallFunction|HandlingExplosion))))

(fn ConstructionScript)

(fn HandlingExplosion
  (Audio|PlaySoundatLocation "/Game/Assets/Sounds/Abilities/ArcaneShards/wav/SFX_RockSpikes_06.SFX_RockSpikes_06" (Transformation|GetActorLocation (Variables|Default|GetBP_Firebolt)) "0, 0, 0" 1.0 1.0 0.0 0 0 0 0)
  (Game|SpawnActorfromClass "/Game/Blueprints/Actor/Breakable/FieldSystem/BP_FieldSystem.BP_FieldSystem_C" (Math|Transform|MakeTransform (Transformation|GetActorLocation (Variables|Default|GetBP_Firebolt)) "0, 0, 0" "1.000000,1.000000,1.000000") "AlwaysSpawn" "MultiplyWithRoot" 0 0))