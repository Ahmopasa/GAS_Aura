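; BP_MagicCircle is a magic circle actor in the Arcane Shards ability folder that displays a spinning decal.
; Each Tick calls RotateTheCircleDecal, which adds RotationSpeed scaled by delta time to the decal's world roll, leaving pitch and yaw unchanged.
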(event EventBeginPlay)

(event Collision|EventActorBeginOverlap
  (params (OtherActor :type Actor%20Object%20Reference)))

(event EventTick
  (params (DeltaSeconds :type Float%20%28single-precision%29))
  (CallFunction|RotatetheCircleDecal DeltaSeconds))

(fn ConstructionScript)

(fn RotatetheCircleDecal
  (params (DeltaSeconds :type Float%20%28single-precision%29))
  (Variables|Default|SetDeltaSeconds DeltaSeconds)
  (bind _output_get (Variables|Default|SetWorldRotation (Transformation|GetWorldRotation (Variables|Default|GetMagicCircleDecal))))
  (Transformation|SetWorldRotation (Variables|Default|GetMagicCircleDecal) (Math|Rotator|MakeRotator (+ (.roll _output_get) (* (Variables|Default|GetDeltaSeconds) (Variables|Default|GetRotationSpeed))) (.pitch _output_get) (.yaw _output_get)) false false))